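; First-person knife weapon Blueprint that handles cutting and inspecting states through begin/end notify events.
; On Cut, it plays a swing sound and line-traces a short distance forward from the camera supplied by SetInitialStats.
; A hit applies damage, attaches a scratch decal randomly rotated around the surface normal and spawns an impact emitter.
; ReciveImpactInfo exposes the hit flag, which clears when the cut ends.
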(event EventReciveBeginNotify
  (params (OperationName :type Name :default "None"))
  (switch name OperationName
    (:cut
      (Variables|Control|SetisCutting true)
      (CallFunction|CutLogic))
    (:inspect
      (Variables|Control|SetisInspecting true))))

(event EventReciveEndNotify
  (params (OperationName :type Name :default "None"))
  (switch name OperationName
    (:cut
      (Variables|Control|SetisCutting false)
      (Variables|Control|SetisTargetHit false))
    (:inspect
      (Variables|Control|SetisInspecting false))))

(event EventSetInitialStats
  (params (PlayerCamera :type Camera%20Component%20Object%20Reference))
  (Variables|Default|SetFirstPersonCamera PlayerCamera))

(fn ConstructionScript)

(fn CutLogic
  ;[1 1 1] Knife swing sounds player
  (Audio|Components|Audio|SetSound (Variables|Default|GetAudio) "/Game/Assets/Knife_FPS/FPWeapon/Audio/SC_Swings.SC_Swings")
  (Audio|Components|Audio|Play (Variables|Default|GetAudio) 0.0)
  ;[1 1 1] Cut trace calculation logic, spawning cut decal at impact point
  (bind _cutlocation (Utilities|CutTrace)
    (:Output
      (bind (_outhit _returnvalue) (Collision|LineTraceByChannel (Transformation|GetWorldLocation (Variables|Default|GetFirstPersonCamera)) _cutlocation "TraceTypeQuery1" false 0 "None"))
      (if _returnvalue
        (Variables|Control|SetisTargetHit _returnvalue)
        (Game|Damage|ApplyDamage (.HitActor (Collision|BreakHitResult _outhit)) 2e+01 0 self)
        (bind _randomrotator (CallFunction|CreateRandomRotator (.ImpactNormal (Collision|BreakHitResult _outhit))))
        (bind _returnvalue_2 (Class|GameplayStatics|SpawnDecalAttached "/Game/Assets/Knife_FPS/FPWeapon/Materials/M_Scratch.M_Scratch" "6.000000,6.000000,6.000000" (.HitComponent (Collision|BreakHitResult _outhit)) "None" (.Location (Collision|BreakHitResult _outhit)) _randomrotator "KeepWorldPosition" 0.0))
        (Rendering|Components|Decal|SetFadeScreenSize _returnvalue_2 0.0)
        (Effects|SpawnEmitteratLocation 0 (.Location (Collision|BreakHitResult _outhit)) _randomrotator "0.200000,0.200000,0.200000")))))

(fn CreateRandomRotator
  (params (NormalVector :type Vector))
  (bind _returnvalue (Math|Random|RandomFloatinRange -1.8e+02 1.8e+02))
  (bind _returnvalue_2 (Math|Conversions|RotationFromXVector NormalVector))
  (bind (_x _y _z) (Math|Rotator|GetAxes _returnvalue_2))
  ;[1 1 1] Random decal rotation logic
  (return (Math|Rotator|MakeRotationfromAxes _x (Math|Vector|RotateVectorAroundAxis _y _returnvalue _x) (Math|Vector|RotateVectorAroundAxis _z _returnvalue _x))))

(fn ReciveImpactInfo
  (return (Variables|Control|GetisTargetHit)))