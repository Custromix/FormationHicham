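; BP_TriggerFinalBossBattle is a placed trigger volume that starts the final boss battle when the player enters it.
; On BeginPlay it caches the main game mode, GM_MainGameMode.
; When a pawn controlled by the first player controller overlaps its Box, it calls RequestFinalBossStart on that game mode.
; The trigger destroys itself only if the request returns true, so a refused request leaves it in place for another attempt.
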(event OnComponentBeginOverlap(Box)
  (params (OverlappedComponent :type Primitive%20Component%20Object%20Reference) (OtherActor :type Actor%20Object%20Reference) (OtherComp :type Primitive%20Component%20Object%20Reference) (OtherBodyIndex :type Integer) (bFromSweep :type Boolean) (SweepResult :type Hit%20Result%20Structure%20%28by%20ref%29))
  (bind _aspawn (Utilities|Casting|CastToPawn OtherActor))
  (if (== (Game|GetPlayerController 0) (Pawn|GetController _aspawn))
    (bind _returnvalue (Class|FormationTestGameMode|RequestFinalBossStart (Variables|Default|GetGM%20Main%20Game%20Mode)))
    (if _returnvalue
      (Actor|DestroyActor))))

(event EventBeginPlay
  (bind _asgm_main_game_mode (Utilities|Casting|CastToGM_MainGameMode (Game|GetGameMode)))
  (Variables|Default|SetGM%20Main%20Game%20Mode _asgm_main_game_mode))

(event Collision|EventActorBeginOverlap
  (params (OtherActor :type Actor%20Object%20Reference)))

(event EventTick
  (params (DeltaSeconds :type Float%20%28single-precision%29)))

(fn ConstructionScript)