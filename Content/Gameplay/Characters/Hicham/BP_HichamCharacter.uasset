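; BP_HichamCharacter is a character Blueprint that starts play with a knife equipped and adds a HUD widget to the player screen.
; When AvoidanceType is SceneComponent2D, the construction script makes the first-person mesh scene-capture-only and registers it with SceneCaptureComponent2D, otherwise hiding that component.
; Item switches do the same for the equipped item's mesh, rendering the first-person view separately, apparently to avoid clipping.
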(event Custom|OnItemSwitch_Event
  (params (LHIKTransform :type Transform))
  (if (Utilities|Enum|Equal(Enum) (Variables|Default|GetAvoidanceType) "SceneComponent2D")
    (Class|PrimitiveComponent|SetVisibleinSceneCaptureOnly (Variables|/Script/FormationHicham.Item|GetItemMesh (Variables|Default|GetEquippedItemActor)) true)
    (Rendering|SceneCapture|ShowOnlyComponent (Variables|Default|GetSceneCaptureComponent2D) (Variables|/Script/FormationHicham.Item|GetItemMesh (Variables|Default|GetEquippedItemActor)))))

(event EventBeginPlay
  (EventDispatchers|AssignOnItemSwitch (delegate Custom|OnItemSwitch_Event))
  (Class|HichamCharacter|TryPickupItem "/Game/Gameplay/Items/DataAssets/DAK_Knife.DAK_Knife")
  (Class|HichamCharacter|Equip "/Game/Gameplay/Items/DataAssets/DAK_Knife.DAK_Knife")
  (bind _returnvalue (UserInterface|CreateWidget "/Game/Widget/W_HUD1.W_HUD1_C"))
  (UserInterface|Viewport|AddtoPlayerScreen _returnvalue))

(event EventTick
  (params (DeltaSeconds :type Float%20%28single-precision%29)))

(fn ConstructionScript
  (if (Utilities|Enum|Equal(Enum) (Variables|Default|GetAvoidanceType) "SceneComponent2D")
    (Rendering|SetVisibility (Variables|Default|GetSceneCaptureComponent2D) true false)
    (Class|PrimitiveComponent|SetVisibleinSceneCaptureOnly (Variables|Default|GetCharacterMesh1P) true)
    (Rendering|SceneCapture|ShowOnlyComponent (Variables|Default|GetSceneCaptureComponent2D) (Variables|Default|GetCharacterMesh1P))
    (else
      (Rendering|SetVisibility (Variables|Default|GetSceneCaptureComponent2D) false false))))