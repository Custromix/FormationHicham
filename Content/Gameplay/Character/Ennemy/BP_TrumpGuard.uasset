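; BP_TrumpGuard is an enemy character Blueprint with a floating health bar above it.
; On BeginPlay it casts the widget component's widget to W_HealthBar and hands it the HealthComponent.
; Every Tick it rotates the widget component to face the player camera, so the bar stays readable from any angle.
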(event EventBeginPlay
  (bind _asw_health_bar (Utilities|Casting|CastToW_HealthBar (UserInterface|GetWidget (Variables|Default|GetWidget))))
  (Default|SetupHealth _asw_health_bar (Variables|Default|GetHealthComponent)))

(event Collision|EventActorBeginOverlap
  (params (OtherActor :type Actor%20Object%20Reference)))

(event EventTick
  (params (DeltaSeconds :type Float%20%28single-precision%29))
  (Transformation|SetWorldRotation (Variables|Default|GetWidget) (Math|Rotator|FindLookatRotation (Transformation|GetWorldLocation (Variables|Default|GetWidget)) (Transformation|GetWorldLocation (Variables|/Script/Engine.PlayerCameraManager|GetTransformComponent (Game|GetPlayerCameraManager 0)))) false false))

(fn ConstructionScript)